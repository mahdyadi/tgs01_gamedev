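; Level teleporter actor that moves the player to NextLevel once its PoponiumList is empty.
; On BeginPlay it registers itself with the player's HUD widget as LvlTeleporter.
; When the player overlaps it with the list empty, it spawns a particle effect near them, waits briefly, then opens the level.
; RemovePoponium takes destroyed Poponium out of the list with debug prints; Tick only casts the player pawn.
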(event `self.ReceiveBeginPlay`
  (bind _asplayer_2 (cast `/Game/Blueprints/player2` (`GameplayStatics.GetPlayerPawn` 0)))
  (bind _ashud (cast `/Game/UI/HUD` (`/Game/Blueprints/player2.HUD Widget` _asplayer_2)))
  (set `/Game/UI/HUD.LvlTeleporter` self _ashud))

(event `self.ReceiveActorBeginOverlap`
  (params (OtherActor :type "Actor Object Reference"))
  (bind _returnvalue (`GameplayStatics.GetPlayerPawn` 0))
  (bind _returnvalue_2 (`self.GetTransform` _returnvalue))
  (if (== OtherActor _returnvalue)
    (if (== (`KismetArrayLibrary.Array_Length` (`self.poponium list`)) 0)
      (`GameplayStatics.SpawnEmitterAtLocation` "/Game/Sprites/ParticleTest.ParticleTest" (`KismetMathLibrary.MakeVector` (.x (.location _returnvalue_2)) 2.0 (- (.z (.location _returnvalue_2)) 5.0)) (struct :`Pitch` 90.0))
      (`KismetSystemLibrary.Delay` 1.0)
      (`GameplayStatics.OpenLevel` (`self.Next level`)))))

(event `self.ReceiveTick`
  (params (DeltaSeconds :type "Float (single-precision)"))
  (bind _asplayer_2 (cast `/Game/Blueprints/player2` (`GameplayStatics.GetPlayerPawn` 0))))

(fn `removePoponium`
  (params (destroyedPoponium :type "/Game/Blueprints/EnvActor/poponium Object Reference"))
  (bind _returnvalue (`KismetArrayLibrary.Array_RemoveItem` (`self.poponium list`) destroyedPoponium))
  (if _returnvalue
    (`KismetSystemLibrary.PrintString` (`KismetSystemLibrary.GetDisplayName` destroyedPoponium))
    (else
      (`KismetSystemLibrary.PrintString` "gagal"))))

(fn `UserConstructionScript`)