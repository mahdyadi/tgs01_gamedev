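; Red robot enemy for a sprite-based side-scroller that patrols around its spawn point and shoots at the player.
; Tick checks player distance: when far, a looping timeline offsets X, and movement deltas drive facing and sprite playback.
; Within 800 units it stops patrolling and faces the player.
; Within 600 it spawns bullets pitched toward the player, throttled by a DoOnce with delayed reset, with debug prints left in.
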(event `UpdateAnimation`
  (bind _returnvalue_x (`KismetMathLibrary.BreakVector` (`self.K2_GetActorLocation`)))
  (bind _momentloc_x (`KismetMathLibrary.BreakVector` (`self.MomentLoc`)))
  (bind _returnvalue (- _returnvalue_x _momentloc_x))
  (`|ExecutionSequence`
    (:`then_0`
      (`KismetSystemLibrary.PrintString` (`KismetStringLibrary.Conv_DoubleToString` _returnvalue) true true (struct :`G` 0.66 :`B` 1.0 :`A` 1.0) 0.0)
      (if (> _returnvalue 0.5)
        (set `self.charState` "NewEnumerator1")
        (`self.K2_SetActorRotation` (struct))
        (`CharacterMovementComponent.SetMovementMode` (`self.CharacterMovement`) "MOVE_NavWalking" 0 :!label _label)
        (elif (< _returnvalue -0.5)
          (set `self.charState` "NewEnumerator1")
          (`self.K2_SetActorRotation` (struct :`Yaw` 180.0))
          (goto _label)
          (else
            (set `self.charState` "NewEnumerator0")))))
    (:`then_1`
      (switch `/Game/Blueprints/Enum_CharState` (`self.charState`)
        (:`NewEnumerator0`
          (`PaperFlipbookComponent.Stop` (`self.Sprite`)))
        (:`NewEnumerator1`
          (`PaperFlipbookComponent.Play` (`self.Sprite`)))))))

(event `self.ReceiveTick`
  (params (DeltaSeconds :type "Float (single-precision)"))
  (bind _returnvalue (`KismetMathLibrary.VSize` (`self.PlayerDistance`)))
  (`|ExecutionSequence`
    (:`then_0`
      (bind _output_get (set `self.Actorloc` (`self.K2_GetActorLocation`)))
      (set `self.PlayerDistance` (- (`self.K2_GetActorLocation` (`GameplayStatics.GetPlayerPawn` 0)) _output_get)))
    (:`then_1`
      (if (< _returnvalue 800.0)
        (`self.StopRoutine`)
        (`self.LookForPlayer`)
        (else
          (`self.Routine`))))
    (:`then_2`
      (if (< _returnvalue 600.0)
        (`KismetSystemLibrary.PrintString` "tembak")
        (`self.Shoot`)))
    (:`then_3`
      (set `self.MomentLoc` (`self.K2_GetActorLocation`)))))

(event `self.ReceiveBeginPlay`
  (bind _output_get (set `self.InitActorLoc` (`self.K2_GetActorLocation`)))
  (set `self.MomentLoc` _output_get))

(event `LookForPlayer`
  (bind _returnvalue_location (`KismetMathLibrary.BreakTransform` (`self.GetTransform`)))
  (bind _returnvalue_location_2 (`KismetMathLibrary.BreakTransform` (`self.GetTransform` (`GameplayStatics.GetPlayerPawn` 0))))
  (bind _output_get (set `self.PlayerDistance` (- _returnvalue_location_2 _returnvalue_location)))
  (if (< (.x _output_get) 0.0)
    (`self.K2_SetActorRotation` (`KismetMathLibrary.MakeRotator` 0.0 0.0 180.0))
    (elif (> (.x _output_get) 0.0)
      (`self.K2_SetActorRotation` (`KismetMathLibrary.MakeRotator` 0.0 0.0 0.0)))))

(event `Shoot`
  (bind _returnvalue (`SceneComponent.K2_GetComponentToWorld` (`self.ShootPoint`)))
  (bind (_returnvalue_roll _returnvalue_pitch) (`KismetMathLibrary.BreakRotator` (`KismetMathLibrary.FindLookAtRotation` (.location _returnvalue) (`self.K2_GetActorLocation` (`GameplayStatics.GetPlayerPawn` 0)))))
  (`/Engine/EditorBlueprintResources/StandardMacros.DoOnce` false :!label _label_2
    (:`Completed`
      (`|SpawnActorFromClass` "/Game/Blueprints/EnemyBullet.EnemyBullet_C" (`KismetMathLibrary.MakeTransform` (.location _returnvalue) (`KismetMathLibrary.MakeRotator` 0.0 _returnvalue_pitch (.yaw (.rotation _returnvalue)))) "Undefined" "OverrideRootScale")
      (`KismetSystemLibrary.Delay` 0.5)
      (goto _label_2 :!via `Reset`))))

(event `Routine`
  (bind (_initactorloc_x _initactorloc_y _initactorloc_z) (`KismetMathLibrary.BreakVector` (`self.InitActorLoc`)))
  (bind (_direction _newtrack_0) (`Timeline|Timeline_0` :!label _label_3)
    (:`Update`
      (`self.K2_SetActorLocation` (`KismetMathLibrary.MakeVector` (+ _initactorloc_x _newtrack_0) _initactorloc_y _initactorloc_z))
      (`self.UpdateAnimation`))
    (:`Finished`
      (`KismetSystemLibrary.Delay` 0.1)
      (goto _label_3 :!via `PlayFromStart`))))

(event `StopRoutine`
  (goto _label_3 :!via `Stop`))

(fn `UserConstructionScript`)