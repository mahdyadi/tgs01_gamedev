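; Level exit teleporter actor that moves the player to the next level once every Poponium is gone.
; When the player pawn overlaps it and its Poponium list is empty, it opens the configured NextLevel by name.
; RemovePoponium takes a destroyed Poponium out of the list and prints its name, or a failure message if it was not found.
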(event `self.ReceiveActorBeginOverlap`
  (params (OtherActor :type "Actor Object Reference"))
  (if (== OtherActor (`GameplayStatics.GetPlayerPawn` 0))
    (if (== (`KismetArrayLibrary.Array_Length` (`self.poponium list`)) 0)
      (`GameplayStatics.OpenLevel` (`self.Next level`)))))

(fn `removePoponium`
  (params (destroyedPoponium :type "/Game/Blueprints/poponium Object Reference"))
  (bind _returnvalue (`KismetArrayLibrary.Array_RemoveItem` (`self.poponium list`) destroyedPoponium))
  (if _returnvalue
    (`KismetSystemLibrary.PrintString` (`KismetSystemLibrary.GetDisplayName` destroyedPoponium))
    (else
      (`KismetSystemLibrary.PrintString` "gagal"))))

(fn `UserConstructionScript`)